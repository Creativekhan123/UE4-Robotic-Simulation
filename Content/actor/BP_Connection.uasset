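; BP_Connection is an actor that opens and manages a serial COM port connection using settings entered in a widget.
; On BeginPlay it shows WB_Connection with the mouse cursor, and its Okay button opens the port from the widget's port and baud rate.
; On success it stores the connection, removes the widget and calls OnPortOpen.
; A separate event sends a hardcoded test JSON line, and EndPlay closes the port.
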(event Custom|Open%20Connection
  (bind _wb_connection (Variables|Default|GetWB_Connection))
  (Utilities|IsValid _wb_connection
    (:Is%20Valid
      (bind (_bopened _returnvalue) (Class|SerialCom|OpenComPort (Variables|/Game/Widgets/WB_Connection.WB_Connection_C|GetPortNumber _wb_connection) (Variables|/Game/Widgets/WB_Connection.WB_Connection_C|GetBondRate _wb_connection)))
      (if _bopened
        (Variables|Default|SetConnection _returnvalue)
        (Widget|RemovefromParent (Variables|Default|GetWB_Connection))
        (Variables|/Script/Engine.PlayerController|SetbShowMouseCursor (Game|GetPlayerController 0) (Variables|Default|GetSHOW_MOUSE))
        (Default|CallOnPortOpen)
        (else
          (Development|PrintString "Fail to open the port"))))
    (:Is%20Not%20Valid
      (Development|PrintString "Connection Object is not valid"))))

(event Custom|sendJson
  (bind _returnvalue (Class|SerialCom|Println (Variables|Default|GetConnection) "{\"name\": \"Zeeshan\",\"age\":12}"))
  (if _returnvalue
    (Development|PrintString "Json has been sended")))

(event EventBeginPlay
  (bind _returnvalue (UserInterface|CreateWidget "/Game/Widgets/WB_Connection.WB_Connection_C"))
  (bind _output_get (Variables|Default|SetWB_Connection _returnvalue))
  (UserInterface|Viewport|AddtoViewport _returnvalue 0)
  (EventDispatchers|BindEventtoOkayButtonClicked _output_get (delegate Custom|Open%20Connection))
  (Variables|/Script/Engine.PlayerController|SetbShowMouseCursor (Game|GetPlayerController 0) true))

(event EventEndPlay
  (params (EndPlayReason :type EEndPlayReason%20Enum :default "Destroyed"))
  (bind _connection (Variables|Default|GetConnection))
  (Utilities|IsValid _connection
    (:Is%20Valid
      (Class|SerialCom|Close _connection))))

(fn ConstructionScript)